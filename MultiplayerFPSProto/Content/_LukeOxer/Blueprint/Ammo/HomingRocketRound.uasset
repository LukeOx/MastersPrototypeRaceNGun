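; Homing rocket projectile that deals area damage on impact and can be told to track a given actor.
; SetupHoming enables projectile homing and adds a new static mesh component to the target actor to serve as the homing target.
; On hitting anything but the first-person character, a sphere trace on Visibility, ignoring the player, damages each hit actor.
; The impact effect and self-destruction occur only when that trace finds something.
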(event `self.ReceiveHit`
  (params (MyComp :type "PrimitiveComponent Object Reference") (Other :type "Actor Object Reference") (OtherComp :type "PrimitiveComponent Object Reference") (bSelfMoved :type Boolean) (HitLocation :type "Vector Structure") (HitNormal :type "Vector Structure") (NormalImpulse :type "Vector Structure") (Hit :type "HitResult Structure (by ref)"))
  (bind _returnvalue (`self.K2_GetActorLocation`))
  (if (!= (`GameplayStatics.GetObjectClass` Other) "/Game/Characters/Blueprints/FirstPersonCharacter.FirstPersonCharacter_C")
    (bind (_outhits _returnvalue_2) (`KismetSystemLibrary.SphereTraceMulti` _returnvalue _returnvalue 50.0 "TraceTypeQuery1" false (`|MakeArray` (`GameplayStatics.GetPlayerCharacter` 0) :!type "Actor Object Reference")))
    (if _returnvalue_2
      (for _array_element _outhits
        (`GameplayStatics.ApplyDamage` (`.HitActor` (`GameplayStatics.BreakHitResult` _array_element)) 25.0))
      (`NiagaraFunctionLibrary.SpawnSystemAtLocation` "/Game/_LukeOxer/FX/RocketHit.RocketHit" _returnvalue)
      (`self.K2_DestroyActor`))))

(event `SetupHoming`
  (params (Actor :type "Actor Object Reference"))
  (bind _projectile (`self.Projectile`))
  (set `ProjectileMovementComponent.bIsHomingProjectile` true _projectile)
  (bind _returnvalue (`AddComponent|NODE_AddStaticMeshComponent-0` :`self` Actor))
  (set `ProjectileMovementComponent.HomingTargetComponent` _returnvalue _projectile))

(fn `UserConstructionScript`)