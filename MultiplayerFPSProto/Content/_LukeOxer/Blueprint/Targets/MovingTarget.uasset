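; MovingTarget is a damageable target actor that shuttles back and forth between its first two waypoints.
; Two timelines drive a position lerp, one forward and one reversed, chaining into each other with a short pause at each end.
; Damage lowers clamped Health shown on a TextRender; at zero the cube hides and drops collision, then returns at full health after a delay.
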(event `self.ReceiveBeginPlay`
  (bind _waypoints (`self.Waypoints`))
  (bind _returnvalue (`self.K2_GetActorLocation` (`|GetArrayItem` _waypoints)))
  (bind _returnvalue_2 (`self.K2_GetActorLocation` (`|GetArrayItem` _waypoints 1)))
  (bind (_direction _alpha) (`Timeline|Lerp` :!label _label)
    (:`Update`
      (`self.K2_SetActorLocation` (`KismetMathLibrary.VLerp` _returnvalue _returnvalue_2 _alpha)))
    (:`Finished`
      (`KismetSystemLibrary.Delay` 0.2)
      (bind (_direction_2 _alpha_2) (`Timeline|Timeline_0` :!via `ReverseFromEnd`)
        (:`Update`
          (`self.K2_SetActorLocation` (`KismetMathLibrary.VLerp` _returnvalue _returnvalue_2 _alpha_2)))
        (:`Finished`
          (`KismetSystemLibrary.Delay` 0.2)
          (goto _label :!via `PlayFromStart`))))))

(event `self.ReceiveAnyDamage`
  (params (Damage :type "Float (single-precision)") (DamageType :type "DamageType Object Reference") (InstigatedBy :type "Controller Object Reference") (DamageCauser :type "Actor Object Reference"))
  (bind _cube (`self.Cube`))
  (bind _output_get (set `self.Health` (`KismetMathLibrary.FClamp` (- (`self.Health`) Damage) 0.0 100.0)))
  (`TextRenderComponent.K2_SetText` (`self.TextRender`) (`KismetTextLibrary.Conv_DoubleToText` _output_get "HalfToEven"))
  (if (<= (`self.Health`) 0.0)
    (`PrimitiveComponent.SetCollisionEnabled` _cube "NoCollision")
    (`SceneComponent.SetVisibility` _cube false false)
    (`KismetSystemLibrary.Delay` 5.0)
    (`PrimitiveComponent.SetCollisionEnabled` _cube "QueryAndPhysics")
    (`SceneComponent.SetVisibility` _cube true false)
    (bind _output_get_2 (set `self.Health` 100.0))
    (`TextRenderComponent.K2_SetText` (`self.TextRender`) (`KismetTextLibrary.Conv_DoubleToText` _output_get_2 "HalfToEven"))))

(fn `UserConstructionScript`
  (`TextRenderComponent.K2_SetText` (`self.TextRender`) (`KismetTextLibrary.Conv_DoubleToText` (`self.Health`) "HalfToEven")))