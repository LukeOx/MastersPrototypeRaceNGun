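; AdaptCar is a drivable car that switches between Road, Dirt and Ice tire types, with toggleable first-person and chase cameras.
; Q and E cycle tires, updating the UI, mesh linear damping and physical-material overrides on Dirt and Ice surface actors.
; Dirt tires make dirt act as road; Ice tires do so for both surfaces, with more damping.
; Possession creates the CarUI and a looping timer that updates the speed dial and brake input.
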(event `/Game/Characters/Blueprints/PawnInterface.MoveRight`
  (params (AxisValue :type "Float (single-precision)"))
  (`WheeledVehicleMovementComponent.SetSteeringInput` (`self.VehicleMovement`) AxisValue))

(event `/Game/Characters/Blueprints/PawnInterface.MoveForward`
  (params (AxisValue :type "Float (single-precision)"))
  (`WheeledVehicleMovementComponent.SetThrottleInput` (`self.VehicleMovement`) AxisValue))

(event `Key|V`
  (params (Key :type "Key Structure"))
  (bind _chase_cam (`self.Chase_Cam`))
  (bind _fp_cam (`self.FP_Cam`))
  (:`Pressed`
    (`/Engine/EditorBlueprintResources/StandardMacros.FlipFlop`
      (:`A`
        (`ActorComponent.Activate` _fp_cam false)
        (`ActorComponent.Deactivate` _chase_cam))
      (:`B`
        (`ActorComponent.Activate` _chase_cam false)
        (`ActorComponent.Deactivate` _fp_cam)))))

(event `self.ReceivePossessed`
  (params (NewController :type "Controller Object Reference"))
  (bind _returnvalue (`KismetSystemLibrary.K2_SetTimerDelegate` (delegate `UpdateSpeed`) 0.01 true))
  (bind _returnvalue_2 (`|CreateWidget` "/Game/_LukeOxer/Blueprint/UI/CarUI.CarUI_C" (`GameplayStatics.GetPlayerController` 0)))
  (bind _output_get (set `self.UI` _returnvalue_2))
  (`UserWidget.AddToViewport` _output_get 0))

(event `self.ReceiveUnpossessed`
  (params (OldController :type "Controller Object Reference"))
  (`KismetSystemLibrary.K2_ClearAndInvalidateTimerHandle` (stale `self.ReceivePossessed` _returnvalue))
  (`Widget.RemoveFromParent` (`self.UI`)))

(event `UpdateSpeed`
  (`/Game/_LukeOxer/Blueprint/UI/CarUI.SetSpeedDialValue` (`self.UI`) (/ (`KismetMathLibrary.VSize` (`self.GetVelocity`)) 2152.0))
  (`WheeledVehicleMovementComponent.SetBrakeInput` (`self.VehicleMovement`) (`self.BrakeMod`)))

(event `/Game/Characters/Blueprints/PawnInterface.Q`
  (bind _dirt (`self.Dirt`))
  (bind _ice (`self.Ice`))
  (bind _mesh (`self.Mesh`))
  (bind _ui (`self.UI`))
  (bind _result (`/Engine/EditorBlueprintResources/StandardMacros.DecrementInt` (`self.TireValue`))
    (:`  `
      (if (< _result 0)
        (set `self.TireValue` 2))
      (switch `int` (`self.TireValue`) :!label _label
        (:`0`
          (set `/Game/_LukeOxer/Blueprint/UI/CarUI.Type` "Road" _ui)
          (`PrimitiveComponent.SetLinearDamping` _mesh 0.01)
          (`|ExecutionSequence`
            (:`then_0`
              (for _array_element _dirt
                (`PrimitiveComponent.SetPhysMaterialOverride` (`self.GetComponentByClass` _array_element "/Script/Engine.PrimitiveComponent") "/Game/_LukeOxer/Blueprint/PhysicsMaterials/Dirt.Dirt")))
            (:`then_1`
              (for _array_element_2 _ice :!label _label_2
                (`PrimitiveComponent.SetPhysMaterialOverride` (`self.GetComponentByClass` _array_element_2 "/Script/Engine.PrimitiveComponent") "/Game/_LukeOxer/Blueprint/PhysicsMaterials/Ice.Ice")))))
        (:`1`
          (set `/Game/_LukeOxer/Blueprint/UI/CarUI.Type` "Dirt" _ui)
          (`PrimitiveComponent.SetLinearDamping` _mesh 0.1)
          (`|ExecutionSequence`
            (:`then_0`
              (goto _label_2))
            (:`then_1`
              (for _array_element_3 _dirt :!label _label_3
                (`PrimitiveComponent.SetPhysMaterialOverride` (`self.GetComponentByClass` _array_element_3 "/Script/Engine.PrimitiveComponent") "/Game/_LukeOxer/Blueprint/PhysicsMaterials/Road.Road")))))
        (:`2`
          (set `/Game/_LukeOxer/Blueprint/UI/CarUI.Type` "Ice" _ui)
          (`PrimitiveComponent.SetLinearDamping` _mesh 0.25)
          (`|ExecutionSequence`
            (:`then_0`
              (goto _label_3))
            (:`then_1`
              (for _array_element_4 _ice
                (`PrimitiveComponent.SetPhysMaterialOverride` (`self.GetComponentByClass` _array_element_4 "/Script/Engine.PrimitiveComponent") "/Game/_LukeOxer/Blueprint/PhysicsMaterials/Road.Road")))))))))

(event `/Game/Characters/Blueprints/PawnInterface.E`
  (bind _result (`/Engine/EditorBlueprintResources/StandardMacros.IncrementInt` (`self.TireValue`))
    (:`  `
      (if (> _result 2)
        (set `self.TireValue` 0)
        (goto _label)
        (else
          (goto _label))))))

(fn `GetHealth`
  (returns (Return :type "Float (double-precision)"))
  (return 0.0))

(fn `GetWeaponActorRef`
  (returns (Return :type "Actor Object Reference"))
  (return null))

(fn `UserConstructionScript`)