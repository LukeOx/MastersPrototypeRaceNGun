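; WeaponFactory is a respawning weapon pickup that gives its configured WeaponClass to any FirstPersonCharacter overlapping its sphere.
; The construction script reads that class's defaults to set the floating skeletal mesh and tint a dynamic material's BodyColor to the weapon colour.
; After collection, it hides the mesh and disables sphere collision, then restores both once RespawnTime elapses.
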(event `SetCollectability`
  (params (Enabled :type Boolean))
  (`SceneComponent.SetVisibility` (`self.FloatingMesh`) Enabled false)
  (`PrimitiveComponent.SetCollisionEnabled` (`self.Sphere`) (select `bool` Enabled :`false` "NoCollision" :`true` "QueryOnly" :!type "ECollisionEnabled Enum")))

(event `self.Sphere.OnComponentBeginOverlap`
  (params (OverlappedComponent :type "PrimitiveComponent Object Reference") (OtherActor :type "Actor Object Reference") (OtherComp :type "PrimitiveComponent Object Reference") (OtherBodyIndex :type Integer) (bFromSweep :type Boolean) (SweepResult :type "HitResult Structure (by ref)"))
  (bind _asfirst_person_character (cast `/Game/Characters/Blueprints/FirstPersonCharacter` OtherActor))
  (`/Game/Characters/Blueprints/FirstPersonCharacter.CollectWeapon` _asfirst_person_character (`self.WeaponClass`))
  (`self.SetCollectability` false)
  (`KismetSystemLibrary.Delay` (`self.RespawnTime`))
  (`self.SetCollectability` true))

(fn `UserConstructionScript`
  (bind _floatingmesh (`self.FloatingMesh`))
  (bind (_primarycanpartfire _weaponorder _basedamage _secondaryfireonrelease _secondarydamage _secondarycanpartfire _pickupmesh _ammomesh _weaponowner _weaponcolour) (defaults `Object` (`self.WeaponClass`)))
  (`SkinnedMeshComponent.SetSkinnedAssetAndUpdate` _floatingmesh (`|ConvertAsset` _pickupmesh) true)
  (bind _returnvalue (`PrimitiveComponent.CreateDynamicMaterialInstance` _floatingmesh 0 (`PrimitiveComponent.GetMaterial` _floatingmesh 0) "None"))
  (`MaterialInstanceDynamic.SetVectorParameterValue` _returnvalue "BodyColor" _weaponcolour))