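; Jump pad actor that launches any Character overlapping its box upward and plays a sound at the pad.
; Vertical velocity scales with JumpPadStrength; with UseTarget, TargetLocation's X and Y serve directly as horizontal velocity, without an arc calculation.
; The construction script moves a sphere to the target offset, or hides it in game when targeting is off.
; A disconnected ballistic-arc launch calculation remains in the graph but never runs.
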(event `self.Box.OnComponentBeginOverlap`
  (params (OverlappedComponent :type "PrimitiveComponent Object Reference") (OtherActor :type "Actor Object Reference") (OtherComp :type "PrimitiveComponent Object Reference") (OtherBodyIndex :type Integer) (bFromSweep :type Boolean) (SweepResult :type "HitResult Structure (by ref)"))
  (bind _returnvalue (* 1000 (`self.JumpPadStrength`)))
  (bind _ascharacter (cast `Character` OtherActor))
  (`Character.LaunchCharacter` _ascharacter (select `bool` (`self.UseTarget`) :`false` (`KismetMathLibrary.MakeVector` 0.0 0.0 _returnvalue) :`true` (`KismetMathLibrary.MakeVector` (.x (`self.TargetLocation`)) (.y (`self.TargetLocation`)) _returnvalue)) (`self.IgnoreInitialVelocityXY`) (`self.IgnoreInitialVelocityZ`))
  (`GameplayStatics.PlaySoundAtLocation` "/Engine/VREditor/Sounds/VR_teleport.VR_teleport" (`self.K2_GetActorLocation`) (struct) 1.0 1.0 0.0 null null null) ; Play firing sound
)

(fn `UserConstructionScript`
  (bind _sphere (`self.Sphere`))
  (if (`self.UseTarget`)
    (`SceneComponent.K2_SetWorldLocation` _sphere (+ (`self.TargetLocation`) (`self.K2_GetActorLocation`)) false false)
    (else
      (`SceneComponent.SetHiddenInGame` _sphere true false))))