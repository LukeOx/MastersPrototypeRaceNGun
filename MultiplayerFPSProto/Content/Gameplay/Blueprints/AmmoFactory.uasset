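; AmmoFactory is a respawning pickup that gives primary or secondary ammo for a configured weapon class.
; The construction script takes the mesh, colour and debug label from the weapon's class defaults, tinting through a dynamic material instance.
; On sphere overlap, a first-person character that owns the weapon collects the ammo.
; The pickup then hides and disables collision until the respawn delay ends, while RotatingMovement targets only the mesh.
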(event `self.ReceiveBeginPlay`
  (`MovementComponent.SetUpdatedComponent` (`self.RotatingMovement`) (`self.StaticMesh`)) ; Updates Root component by default
)

(event `SetCollectability`
  (params (Enabled :type Boolean))
  (`SceneComponent.SetVisibility` (`self.StaticMesh`) Enabled false)
  (`PrimitiveComponent.SetCollisionEnabled` (`self.Sphere`) (select `bool` Enabled :`false` "NoCollision" :`true` "QueryOnly" :!type "ECollisionEnabled Enum"))
  (`SceneComponent.SetVisibility` (`self.DebugEditorText`) Enabled false))

(event `self.Sphere.OnComponentBeginOverlap`
  (params (OverlappedComponent :type "PrimitiveComponent Object Reference") (OtherActor :type "Actor Object Reference") (OtherComp :type "PrimitiveComponent Object Reference") (OtherBodyIndex :type Integer) (bFromSweep :type Boolean) (SweepResult :type "HitResult Structure (by ref)"))
  (bind _weaponid (`self.WeaponID`))
  (bind _givesecondaryammo (`self.GiveSecondaryAmmo`))
  (bind _asfirst_person_character (cast `/Game/Characters/Blueprints/FirstPersonCharacter` OtherActor))
  (if (`/Game/Characters/Blueprints/FirstPersonCharacter.IsValidWeapon` _asfirst_person_character _weaponid)
    (`/Game/Characters/Blueprints/FirstPersonCharacter.CollectAmmo` _asfirst_person_character _weaponid (`KismetMathLibrary.SelectInt` 0 (`self.AmmoToGive`) _givesecondaryammo) (`KismetMathLibrary.SelectInt` (`self.AmmoToGive`) 0 _givesecondaryammo))
    (`self.SetCollectability` false)
    (`KismetSystemLibrary.Delay` (`self.RespawnTime`))
    (`self.SetCollectability` true)))

(fn `UserConstructionScript`
  (bind (_primarycanpartfire _ammoperfire _clipsize _weaponname _weaponorder _fireonrelease _basedamage _fireratetime _reloadtime _hassecondaryammo _secondaryfireonrelease _secondarydamage _secondarycanpartfire _pickupmesh _ammomesh _weaponowner _startingammo _maxammo _ammoperaltfire _secondarystartingammo _secondarymaxammo _weaponcolour) (defaults `Object` (`self.WeaponID`)))
  (`StaticMeshComponent.SetStaticMesh` (`self.StaticMesh`) (`|ConvertAsset` _ammomesh))
  (bind _returnvalue (`PrimitiveComponent.CreateDynamicMaterialInstance` (`self.StaticMesh`) 0 "/Game/DevAssets/M_DynamicColour.M_DynamicColour" "None"))
  (`MaterialInstanceDynamic.SetVectorParameterValue` _returnvalue "Colour" _weaponcolour)
  (`TextRenderComponent.K2_SetText` (`self.DebugEditorText`) (`|FormatText` "{Weapon} \n{Ammo}" _weaponname (`self.AmmoToGive`))))