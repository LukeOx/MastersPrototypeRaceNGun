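; Gameplay player controller that relays input to the controlled pawn through interface messages and handles entering and exiting vehicles.
; Entering sphere-checks for an uncontrolled nearby vehicle, caches the character's weapons, health and weapon index, possesses it and destroys the character.
; Exiting spawns a new character above the pawn, possesses it and restores that state.
; It also creates and refreshes the lobby widget; CreateHUD is an empty stub.
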(event `CreateHUD`)

(event `self.ReceiveBeginPlay`
  (if (`self.IsLocalController`)
    (`self.CreateHUD`)))

(event `ShowLobby`
  (bind _returnvalue (`|CreateWidget` "/Game/UI/Lobby/Lobby.Lobby_C" self))
  (bind _output_get (set `self.LobbyWidget` _returnvalue))
  (`UserWidget.AddToViewport` _output_get 0))

(event `RefreshLobby`
  (`/Game/UI/Lobby/Lobby.Refresh` (stale `ShowLobby` _output_get)))

(event `InputAxis|MoveForward` :consume false :overrideparent false
  (params (AxisValue :type "Float (single-precision)"))
  ;[1 1 1] Pawn Interface
  (message `/Game/Characters/Blueprints/PawnInterface.MoveForward` (`self.K2_GetPawn`) AxisValue))

(event `InputAction|Fire`
  (params (Key :type "Key Structure"))
  (bind _returnvalue (`self.K2_GetPawn`))
  ;[1 1 1] Pawn Interface
  (:`Pressed`
    (message `/Game/Characters/Blueprints/PawnInterface.FirePressed` _returnvalue))
  (:`Released`
    (message `/Game/Characters/Blueprints/PawnInterface.FireReleased` _returnvalue)))

(event `InputAxis|MoveRight` :consume false :overrideparent false
  (params (AxisValue :type "Float (single-precision)"))
  ;[1 1 1] Pawn Interface
  (message `/Game/Characters/Blueprints/PawnInterface.MoveRight` (`self.K2_GetPawn`) AxisValue))

(event `InputAction|AltFire`
  (params (Key :type "Key Structure"))
  (bind _returnvalue (`self.K2_GetPawn`))
  ;[1 1 1] Pawn Interface
  (:`Pressed`
    (message `/Game/Characters/Blueprints/PawnInterface.SecondaryFirePressed` _returnvalue))
  (:`Released`
    (message `/Game/Characters/Blueprints/PawnInterface.SecondaryFireReleased` _returnvalue)))

(event `InputAxis|TurnRate`
  (params (AxisValue :type "Float (single-precision)"))
  ;[1 1 1] Pawn Interface
  (message `/Game/Characters/Blueprints/PawnInterface.TurnRate` (`self.K2_GetPawn`) 0.0))

(event `InputAxis|LookUpRate`
  (params (AxisValue :type "Float (single-precision)"))
  ;[1 1 1] Pawn Interface
  (message `/Game/Characters/Blueprints/PawnInterface.LookUpRate` (`self.K2_GetPawn`) AxisValue))

(event `InputAxis|Turn` :overrideparent false
  (params (AxisValue :type "Float (single-precision)"))
  ;[1 1 1] Pawn Interface
  (message `/Game/Characters/Blueprints/PawnInterface.Turn` (`self.K2_GetPawn`) AxisValue))

(event `InputAction|Reload`
  (params (Key :type "Key Structure"))
  ;[1 1 1] Pawn Interface
  (:`Pressed`
    (message `/Game/Characters/Blueprints/PawnInterface.Reload` (`self.K2_GetPawn`))))

(event `InputAction|WeaponSelect`
  (params (Key :type "Key Structure"))
  ;[1 1 1] Pawn Interface
  (:`Pressed`
    (message `/Game/Characters/Blueprints/PawnInterface.WeaponSelect` (`self.K2_GetPawn`) Key)))

(event `InputAxis|LookUp` :overrideparent false
  (params (AxisValue :type "Float (single-precision)"))
  ;[1 1 1] Pawn Interface
  (message `/Game/Characters/Blueprints/PawnInterface.LookUp` (`self.K2_GetPawn`) AxisValue))

(event `InputAction|Jump` :overrideparent false
  (params (Key :type "Key Structure"))
  (bind _returnvalue (`self.K2_GetPawn`))
  ;[1 1 1] Pawn Interface
  (:`Pressed`
    (message `/Game/Characters/Blueprints/PawnInterface.JumpPressed` _returnvalue))
  (:`Released`
    (message `/Game/Characters/Blueprints/PawnInterface.JumpReleased` _returnvalue)))

(event `InputAction|Interact`
  (params (Key :type "Key Structure"))
  ;[1 1 1] Pawn Interface
  (:`Pressed`
    (cast `/Game/Characters/Blueprints/FirstPersonCharacter` (`self.K2_GetPawn`)
      (:`then`
        (`self.EnterVehicle`))
      (:`CastFailed`
        (`self.ExitVehicle`)))))

(event `ExitVehicle`
  (bind _returnvalue (`self.GetTransform` (`self.K2_GetPawn`)))
  (bind _returnvalue_2 (`|SpawnActorFromClass` "/Game/Characters/Blueprints/FirstPersonCharacter.FirstPersonCharacter_C" (`KismetMathLibrary.MakeTransform` (`KismetMathLibrary.MakeVector` (.x (.location _returnvalue)) (.y (.location _returnvalue)) (+ (.z (.location _returnvalue)) 200.0))) "AdjustIfPossibleButAlwaysSpawn" "OverrideRootScale" null null))
  (`self.UnPossess`)
  (`self.Possess` _returnvalue_2)
  (bind _output_get (set `/Game/Characters/Blueprints/FirstPersonCharacter.Weapons` (`self.CharWeapons`) _returnvalue_2))
  (set `/Game/Characters/Blueprints/FirstPersonCharacter.Health` (`self.CharacterHealth`) _returnvalue_2)
  (`/Game/Characters/Blueprints/FirstPersonCharacter.EquipWeapon` _returnvalue_2 (`.WeaponClass_29_140F200C4C1736CF7C2ABA932B5E209E` (break `/Game/Weapons/Blueprints/WeaponAmmoData` (`|GetArrayItem` _output_get (`self.CharCurrWeapIndex`))))))

(event `InputAxis|FlightHeight`
  (params (AxisValue :type "Float (single-precision)"))
  ;[1 1 1] Pawn Interface
  (message `/Game/Characters/Blueprints/PawnInterface.FlightHeight` (`self.K2_GetPawn`) AxisValue))

(event `Key|Q`
  (params (Key :type "Key Structure"))
  (:`Pressed`
    (message `/Game/Characters/Blueprints/PawnInterface.Q` (`self.K2_GetPawn`))))

(event `EnterVehicle`
  ;[1 1 1] Enter Vehicle
  (bind (_outactors _returnvalue) (`KismetSystemLibrary.SphereOverlapActors` (`self.K2_GetActorLocation` (`self.K2_GetPawn`)) 200.0 (`|MakeArray` "ObjectTypeQuery5" :!type "EObjectTypeQuery Enum")))
  (if _returnvalue
    (bind _output_get (set `self.PlayerCharacter` (cast `/Game/Characters/Blueprints/FirstPersonCharacter` (`self.K2_GetPawn`) :!pure true)))
    (bind _aspawn (cast `Pawn` (`|GetArrayItem` _outactors) :!pure true))
    (`/Engine/EditorBlueprintResources/StandardMacros.IsValid` (`Pawn.GetController` _aspawn)
      (:`Is Not Valid`
        (set `self.CharWeapons` (`/Game/Characters/Blueprints/FirstPersonCharacter.Weapons` _output_get))
        (set `self.CharacterHealth` (`/Game/Characters/Blueprints/FirstPersonCharacter.Health` _output_get))
        (set `self.CharCurrWeapIndex` (`/Game/Characters/Blueprints/FirstPersonCharacter.CurrentWeaponIndex` _output_get))
        (`self.UnPossess`)
        (`self.Possess` _aspawn)
        (`self.K2_DestroyActor` _output_get)))))

(event `Key|E`
  (params (Key :type "Key Structure"))
  (:`Pressed`
    (message `/Game/Characters/Blueprints/PawnInterface.E` (`self.K2_GetPawn`))))

(fn `UserConstructionScript`)