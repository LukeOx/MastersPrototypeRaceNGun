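; Example hitscan weapon Blueprint that extends a parent weapon class by overriding its FireWeapon event.
; After the parent logic, it line-traces on Visibility from the Muzzle socket along the owner's first-person camera direction, ignoring itself and the owner.
; It draws the shot through DrawDebugLineOnAll and applies BaseDamage to the hit actor, crediting the owner as damage causer.
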(event `self.FireWeapon`
  (bind _returnvalue (`SceneComponent.GetSocketLocation` (`self.WeaponMesh`) "Muzzle"))
  (bind _returnvalue_2 (+ _returnvalue (* (`SceneComponent.GetForwardVector` (`/Game/Characters/Blueprints/FirstPersonCharacter.FirstPersonCamera` (`self.WeaponOwner`))) 3000.0)))
  (`parent.FireWeapon`)
  (`self.DrawDebugLineOnAll` _returnvalue _returnvalue_2)
  (bind _outhit (`KismetSystemLibrary.LineTraceSingle` _returnvalue _returnvalue_2 "TraceTypeQuery1" false (`|MakeArray` self (`self.WeaponOwner`) :!type "Actor Object Reference")))
  (`GameplayStatics.ApplyDamage` (`.HitActor` (`GameplayStatics.BreakHitResult` _outhit)) (`self.BaseDamage`) null (`self.WeaponOwner`)))

(fn `UserConstructionScript`
  (`parent.UserConstructionScript`))