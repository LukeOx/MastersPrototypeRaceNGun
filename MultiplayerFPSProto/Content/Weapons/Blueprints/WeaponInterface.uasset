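; Blueprint interface that defines the common contract for weapons.
; It declares press and release inputs for primary and secondary fire, with queries for whether either fire mode or a reload is allowed.
; Ammo is handled as primary held, primary stored and secondary counts, which can be read, set or returned by a reload.
; It also exposes reload time and weapon name, leaving all behavior to implementers.
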(fn `CanPrimaryFire`
  (returns (CanFire :type Boolean))
  (return false))

(fn `CanReload`
  (returns (ReturnValue :type Boolean))
  (return false))

(fn `CanSecondaryFire`
  (returns (CanFire :type Boolean))
  (return false))

(fn `GetAmmo`
  (returns (PrimaryHeld :type Integer) (PrimaryStored :type Integer) (Secondary :type Integer))
  (return 0 0 0))

(fn `GetReloadTime`
  (returns (ReloadTime :type "Float (double-precision)"))
  (return 0.0))

(fn `GetWeaponName`
  (returns (Return :type Name))
  (return "None"))

(fn `PrimaryFire_Pressed`)

(fn `PrimaryFire_Released`)

(fn `SecondaryFire_Pressed`)

(fn `SecondaryFire_Released`)

(fn `SetCurrentAmmoValues`
  (params (PrimaryHeld :type Integer) (PrimaryStored1 :type Integer) (Secondary :type Integer)))

(fn `WeaponReload`
  (returns (NewPrimaryHeld :type Integer) (NewPrimaryStored :type Integer) (NewSecondaryAmmo :type Integer))
  (return 0 0 0))