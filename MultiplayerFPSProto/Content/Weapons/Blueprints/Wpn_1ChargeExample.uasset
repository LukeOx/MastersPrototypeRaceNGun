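; Example charge weapon Blueprint that fires a hitscan shot whose damage scales with how long the charge is held.
; FireWeapon calls the parent, then draws a debug line and runs a Visibility trace from the muzzle socket along the owner's first-person camera direction, ignoring itself and its owner.
; The hit actor takes damage mapped with clamping from ChargeHeld against FireRateTime up to BaseDamage, as a demonstration of the charge variable.
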(event `self.FireWeapon`
  (bind _returnvalue (`SceneComponent.GetSocketLocation` (`self.WeaponMesh`) "Muzzle"))
  (bind _returnvalue_2 (+ _returnvalue (* (`SceneComponent.GetForwardVector` (`/Game/Characters/Blueprints/FirstPersonCharacter.FirstPersonCamera` (`self.WeaponOwner`))) 3000.0)))
  (`parent.FireWeapon`)
  (`self.DrawDebugLineOnAll` _returnvalue _returnvalue_2)
  (bind _outhit (`KismetSystemLibrary.LineTraceSingle` _returnvalue _returnvalue_2 "TraceTypeQuery1" false (`|MakeArray` self (`self.WeaponOwner`) :!type "Actor Object Reference")))
  (`GameplayStatics.ApplyDamage` (`.HitActor` (`GameplayStatics.BreakHitResult` _outhit)) (`KismetMathLibrary.MapRangeClamped` (`self.ChargeHeld`) 0.0 (`self.FireRateTime`) 0.0 (`self.BaseDamage`)) null (`self.WeaponOwner`)))

(fn `UserConstructionScript`
  (`parent.UserConstructionScript`))