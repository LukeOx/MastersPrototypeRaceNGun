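; HeatMapper is an editor-only actor that visualises a set of locations as a heat map on a plane, destroying itself on BeginPlay.
; PaintMarkers spawns attached HeatMarkers, then draws each one's calculated heat colour into a render target through a dynamic material.
; Snapshot exports an orthographic scene capture and the heat map texture as timestamped PNGs, at most once per second.
; RemoveMarkers clears the map and destroys attached markers.
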(event `self.ReceiveBeginPlay`
  (`self.K2_DestroyActor`))

(event `DrawSpicyRenderTarget`
  (params (Location :type "Vector Structure") (Size :type "Float (double-precision)") (HeatColour :type "LinearColor Structure"))
  (bind _textureresolution (`self.TextureResolution`))
  (bind _returnvalue (/ _textureresolution 2.0))
  (bind _returnvalue_x (`KismetMathLibrary.BreakVector` (* (`.BoxExtent` (`KismetSystemLibrary.GetComponentBounds` (`self.Heatmap Plane`))) 2.0)))
  ;[1 1 1] Draw to Render Target
  (`MaterialInstanceDynamic.SetVectorParameterValue` (`self.MI_HeatMapInst`) "HeatColour" HeatColour)
  (`MaterialInstanceDynamic.SetScalarParameterValue` (`self.MI_HeatMapInst`) "Size" Size)
  (`MaterialInstanceDynamic.SetVectorParameterValue` (`self.MI_HeatMapInst`) "Position" (`KismetMathLibrary.Conv_VectorToLinearColor` (/ (+ (* Location (/ (`self.TextureResolution`) _returnvalue_x)) (`KismetMathLibrary.MakeVector` _returnvalue _returnvalue _returnvalue)) _textureresolution)))
  (`KismetRenderingLibrary.DrawMaterialToRenderTarget` (`self.RenderTarget`) (`self.MI_HeatMapInst`)))

(event `PaintMarkers`
  (`self.RemoveMarkers`)
  ;[1 1 1] Get Locations/Create Heat Map
  (for _array_element (`self.Locations`)
    (bind _returnvalue (`|SpawnActorFromClass` "/Game/DevAssets/HeatMap/Blueprints/HeatMarker.HeatMarker_C" (`KismetMathLibrary.MakeTransform` _array_element) "Undefined" "OverrideRootScale" null null))
    (`self.K2_AttachToActor` _returnvalue self "None" "KeepWorld" "KeepWorld" "KeepWorld" true))
  ;[1 1 1] Get Heat Colour & Paint to Render
  (bind _children (`self.HasChildren`)
    (:`true`
      (for _array_element_2 _children
        (bind _asheat_marker (cast `/Game/DevAssets/HeatMap/Blueprints/HeatMarker` _array_element_2))
        (bind _heatcolour (`/Game/DevAssets/HeatMap/Blueprints/HeatMarker.CalculateHeat` _asheat_marker (`self.MaxHeatOverlap`)))
        (`self.DrawSpicyRenderTarget` (`self.K2_GetActorLocation` _asheat_marker) 0.1 _heatcolour))
      (`PrimitiveComponent.SetMaterial` (`self.Heatmap Plane`) 0 "/Game/DevAssets/HeatMap/Materials/ColouredHeatMap.ColouredHeatMap"))))

(event `RemoveMarkers`
  ;[1 1 1] Remove Markers
  (`self.ClearMaps`)
  (bind _children (`self.HasChildren`)
    (:`true`
      (bind _output_get (set `self.TempAttached` _children))
      (for _array_element _output_get
        (`self.K2_DestroyActor` _array_element))
      (`KismetArrayLibrary.Array_Clear` (`self.TempAttached`)))))

(event `Snapshot`
  (bind (_returnvalue_year _returnvalue_month _returnvalue_day _returnvalue_hour _returnvalue_minute _returnvalue_second) (`KismetMathLibrary.BreakDateTime` (`KismetMathLibrary.Now`)))
  (bind _returnvalue (`KismetStringLibrary.Concat_StrStr` (`self.CheckForZero` (`KismetStringLibrary.Conv_IntToString` _returnvalue_hour)) (`self.CheckForZero` (`KismetStringLibrary.Conv_IntToString` _returnvalue_minute)) (`self.CheckForZero` (`KismetStringLibrary.Conv_IntToString` _returnvalue_second)) ".PNG"))
  (bind _returnvalue_2 (`KismetStringLibrary.Concat_StrStr` "HeatMap" _returnvalue))
  (set `SceneCaptureComponent2D.OrthoWidth` (* (`.SphereRadius` (`KismetSystemLibrary.GetComponentBounds` (`self.Heatmap Plane`))) 1.8) (`self.SceneCaptureComponent2D`))
  ;[1 1 1] Export Render Target to File Path
  (if (!= (`self.LastSecond`) _returnvalue_second)
    (set `self.LastSecond` _returnvalue_second)
    (`SceneCaptureComponent2D.CaptureScene` (`self.SceneCaptureComponent2D`))
    (`KismetRenderingLibrary.ExportRenderTarget` "/Game/DevAssets/HeatMap/Textures/ScreenCap.ScreenCap" (`self.FilePath`) _returnvalue_2) ; Note: UE4's viewports have Gamma Correction -- it will be MUCH darker when it's exported!
    (`KismetRenderingLibrary.ExportRenderTarget` "/Game/DevAssets/HeatMap/Textures/HeatmapTarget.HeatmapTarget" (`self.FilePath`) (`KismetStringLibrary.Concat_StrStr` "HeatMap_Tex" _returnvalue))
    (`KismetSystemLibrary.PrintString` (`KismetStringLibrary.Concat_StrStr` "Heat Maps exported to " (`self.FilePath`) "\\" _returnvalue_2) true true (struct :`R` 1.0 :`B` 1.0 :`A` 1.0))
    (else
      (`KismetSystemLibrary.PrintString` "Wait..." true true (struct :`R` 1.0 :`B` 1.0 :`A` 1.0)))))

(event `ClearMaps`
  ;[1 1 1] Clear/Clean maps
  (`KismetRenderingLibrary.ClearRenderTarget2D` (`self.RenderTarget`)) ; Clear Render Target/Map
  (`PrimitiveComponent.SetMaterial` (`self.Heatmap Plane`) 0 "/Game/DevAssets/HeatMap/Materials/TransparentHeatMat.TransparentHeatMat"))

(fn `UserConstructionScript`
  (bind (_returnvalue_x _returnvalue_y _returnvalue_z) (`KismetMathLibrary.BreakVector` (`self.K2_GetActorLocation`)))
  (bind _returnvalue (/ (`self.HeatMapRadius`) 50.0))
  (bind _returnvalue_2 (`KismetMaterialLibrary.CreateDynamicMaterialInstance` "/Game/DevAssets/HeatMap/Materials/HeatMapMat.HeatMapMat"))
  (set `self.MI_HeatMapInst` _returnvalue_2)
  ;[1 1 1] Keep Heat Map in position
  (`self.K2_SetActorLocation` (`KismetMathLibrary.MakeVector` 0.0 0.0 _returnvalue_z))
  (`SceneComponent.K2_SetRelativeLocation` (`self.Heatmap Plane`) (0.0 0.0 0.0) false false)
  ;[1 1 1] Scale Heat Map
  (`SceneComponent.SetWorldScale3D` (`self.Heatmap Plane`) (`KismetMathLibrary.MakeVector` _returnvalue _returnvalue 1.0))
  ;[1 1 1] Set Up Scene Capture
  (set `SceneCaptureComponent2D.OrthoWidth` (* (`self.HeatMapRadius`) 2.0) (`self.SceneCaptureComponent2D`)))