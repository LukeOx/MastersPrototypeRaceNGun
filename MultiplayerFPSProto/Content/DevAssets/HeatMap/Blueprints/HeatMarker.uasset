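; Editor-only heat map marker that shows how densely other HeatMarkers cluster around it, and destroys itself on BeginPlay.
; Construction creates a dynamic material for its sphere.
; CalculateHeat counts other markers overlapping the sphere's bounds and normalises the clamped count against a supplied maximum.
; That ratio is written to the text render and drives a green-to-red material colour, which the function returns.
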(event `self.ReceiveBeginPlay`
  (`self.K2_DestroyActor`))

(fn `CalculateHeat`
  (params (MaxHeatOverlap :type Integer))
  (returns (HeatColour :type "LinearColor Structure"))
  (locals (FloatMax :type "Float (double-precision)" :default 0.0))
  (bind (_origin _boxextent _sphereradius) (`KismetSystemLibrary.GetComponentBounds` (`self.Sphere`)))
  (bind _output_get (set `self.MaxHeatOverlap` MaxHeatOverlap))
  (set `local.FloatMax` (`KismetMathLibrary.Conv_IntToDouble` _output_get))
  (bind _outactors (`KismetSystemLibrary.SphereOverlapActors` _origin _sphereradius (`|MakeArray` "ObjectTypeQuery2" :!type "EObjectTypeQuery Enum") "HeatMarker_C" (`|MakeArray` self :!type "Actor Object Reference")))
  (bind _output_get_2 (set `self.Overlapping` _outactors))
  (bind _returnvalue (/ (`KismetMathLibrary.Conv_IntToDouble` (`KismetMathLibrary.Clamp` (`KismetArrayLibrary.Array_Length` _output_get_2) 0 (`self.MaxHeatOverlap`))) (`local.FloatMax`)))
  (`TextRenderComponent.K2_SetText` (`self.TextRender`) (`KismetTextLibrary.Conv_DoubleToText` _returnvalue "HalfToEven"))
  (bind _output_get_3 (set `self.HeatColour` (`KismetMathLibrary.LinearColorLerp` (struct :`G` 1.0 :`A` 1.0) (struct :`R` 1.0 :`A` 1.0) _returnvalue)))
  (`MaterialInstanceDynamic.SetVectorParameterValue` (`self.HeatMaterial`) "HeatColour" _output_get_3)
  (`KismetArrayLibrary.Array_Clear` (`self.Overlapping`))
  (return _output_get_3))

(fn `UserConstructionScript`
  (bind _sphere (`self.Sphere`))
  (bind _returnvalue (`PrimitiveComponent.CreateDynamicMaterialInstance` _sphere 0 (`PrimitiveComponent.GetMaterial` _sphere 0) "None"))
  (set `self.HeatMaterial` _returnvalue))